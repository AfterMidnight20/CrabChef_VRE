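; Choppable potato for Crab Chef that changes its mesh when struck by a moving melee weapon.
; An overlap on the whole-potato mesh checks for a MeleeBase whose mesh component is moving fast enough to count as a hit.
; A non-looping MultiGate then advances through two static mesh swaps, Cone and BeaconDirection, via a custom event.
; Boundary box overlaps are empty, and older input-toggle and visibility-swap logic is left disconnected.
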(event OnComponentBeginOverlap(Boundary_Box)
  (params (OverlappedComponent :type Primitive%20Component%20Object%20Reference) (OtherActor :type Actor%20Object%20Reference) (OtherComp :type Primitive%20Component%20Object%20Reference) (OtherBodyIndex :type Integer) (bFromSweep :type Boolean) (SweepResult :type Hit%20Result%20Structure%20%28by%20ref%29))
  ;[1 1 1] Boundary for Changing Mesh (Press button)
)

(event OnComponentEndOverlap(Boundary_Box)
  (params (OverlappedComponent :type Primitive%20Component%20Object%20Reference) (OtherActor :type Actor%20Object%20Reference) (OtherComp :type Primitive%20Component%20Object%20Reference) (OtherBodyIndex :type Integer))
  ;[1 1 1] Boundary for Changing Mesh (Press button)
)

(event OnComponentBeginOverlap(Potato_Mesh_Whole)
  (params (OverlappedComponent :type Primitive%20Component%20Object%20Reference) (OtherActor :type Actor%20Object%20Reference) (OtherComp :type Primitive%20Component%20Object%20Reference) (OtherBodyIndex :type Integer) (bFromSweep :type Boolean) (SweepResult :type Hit%20Result%20Structure%20%28by%20ref%29))
  ;[1 1 1] On Melee Base Collission: Change Mesh
  (bind _asmelee_base (Utilities|Casting|CastToMeleeBase OtherActor))
  (if (>= (Math|Vector|VectorLength (Transformation|GetComponentVelocity (Variables|/Script/Engine.StaticMeshActor|GetStaticMeshComponent _asmelee_base))) 1.3e+02)
    (Utilities|FlowControl|MultiGate false false -1
      (:Out%200
        (CallFunction|MeshtoSwitchto "/Engine/BasicShapes/Cone.Cone"))
      (:Out%201
        (CallFunction|MeshtoSwitchto "/Game/VRE/Core/Character/Meshes/BeaconDirection.BeaconDirection")))))

(event Custom|MeshToSwitchTo
  (params (Mesh :type Static%20Mesh%20Object%20Reference))
  ;[1 1 1] SwitchMeshCustomEvent
  (Components|StaticMesh|SetStaticMesh (Variables|Default|GetPotato_Mesh_Whole) Mesh))

(fn ConstructionScript)